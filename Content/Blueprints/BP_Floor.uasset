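; BP_Floor is a floor piece that appears as grass, road or water according to its FloorType.
; On BeginPlay it picks the matching static mesh and gives it a dynamic instance of the shared chicken color material.
; Non-traversable floors are darkened by lowering that instance's "darkness" vector parameter, derived from its red channel, so blocked ground looks different.
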(event EventBeginPlay
  (switch int (Variables|Default|GetFloor%20Type)
    (:0
      (CallFunction|SetMesh "/Game/media/meshes/grass.grass"))
    (:1
      (CallFunction|SetMesh "/Game/media/meshes/road.road"))
    (:2
      (CallFunction|SetMesh "/Game/media/meshes/water.water"))))

(fn ConstructionScript)

(fn DarkenMesh
  (params (Material%20Instance :type Material%20Instance%20Dynamic%20Object%20Reference))
  (bind _returnvalue (Rendering|Material|GetVectorParameterValue Material%20Instance "darkness" :!class /Script/Engine.MaterialInstanceDynamic))
  (Rendering|Material|SetVectorParameterValue Material%20Instance "darkness" (Math|Conversions|ToLinearColor(Float) (- (.R (Utilities|Struct|BreakLinearColor _returnvalue)) 0.4)) :!class /Script/Engine.MaterialInstanceDynamic))

(fn SetMesh
  (params (Static%20Mesh :type Static%20Mesh%20Object%20Reference))
  (Components|StaticMesh|SetStaticMesh (Variables|Default|GetFloor%20Mesh) Static%20Mesh)
  (bind _returnvalue (Rendering|Material|CreateDynamicMaterialInstance (Variables|Default|GetFloor%20Mesh) 0 "/Game/media/meshes/M_chicken__colors_png.M_chicken__colors_png" "None" :!class /Script/Engine.PrimitiveComponent))
  (bind _output_get (Variables|Default|SetMaterial%20Instance _returnvalue))
  (if (not (Variables|Default|GetTraversable))
    (CallFunction|DarkenMesh _output_get)))