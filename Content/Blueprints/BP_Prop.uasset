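; BP_Prop is a static mesh prop that can be shown darkened.
; On BeginPlay it creates a dynamic material instance from the chicken colors material on its mesh and stores it.
; When the Dark flag is set, Darken lowers the material's "darkness" vector parameter, writing back its red channel minus a fixed offset as a color.
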(event EventBeginPlay
  (bind _returnvalue (Rendering|Material|CreateDynamicMaterialInstance (Variables|Default|GetStaticMesh) 0 "/Game/media/meshes/M_chicken__colors_png.M_chicken__colors_png" "None" :!class /Script/Engine.PrimitiveComponent))
  (Variables|Default|SetMaterial%20Instance _returnvalue)
  (if (Variables|Default|GetDark)
    (CallFunction|Darken)))

(fn ConstructionScript)

(fn Darken
  (bind _material_instance (Variables|Default|GetMaterial%20Instance))
  (bind _returnvalue (Rendering|Material|GetVectorParameterValue _material_instance "darkness" :!class /Script/Engine.MaterialInstanceDynamic))
  (Rendering|Material|SetVectorParameterValue _material_instance "darkness" (Math|Conversions|ToLinearColor(Float) (- (.R (Utilities|Struct|BreakLinearColor _returnvalue)) 0.4)) :!class /Script/Engine.MaterialInstanceDynamic))